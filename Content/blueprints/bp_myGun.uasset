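; Pickup actor named as a gun that shows an "장착 [T]" (equip) prompt while something is in range.
; On BeginPlay it writes the prompt into its myPickUpText widget and hides the SmFishingRod2 mesh.
; Sphere overlap begin and end toggle the widget's visibility and the InRange flag, without filtering the overlapping actor.
; The equip input is not handled in this graph.
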(event OnComponentBeginOverlap(Sphere)
  (params (OverlappedComponent :type Primitive%20Component%20Object%20Reference) (OtherActor :type Actor%20Object%20Reference) (OtherComp :type Primitive%20Component%20Object%20Reference) (OtherBodyIndex :type Integer) (bFromSweep :type Boolean) (SweepResult :type Hit%20Result%20Structure%20%28by%20ref%29))
  (Rendering|SetVisibility (Variables|Default|GetWidget) true false)
  (Variables|Default|Setin%20range%20? true))

(event OnComponentEndOverlap(Sphere)
  (params (OverlappedComponent :type Primitive%20Component%20Object%20Reference) (OtherActor :type Actor%20Object%20Reference) (OtherComp :type Primitive%20Component%20Object%20Reference) (OtherBodyIndex :type Integer))
  (Rendering|SetVisibility (Variables|Default|GetWidget) false false)
  (Variables|Default|Setin%20range%20? false))

(event EventBeginPlay
  (bind _asmy_pick_up_text (Utilities|Casting|CastTomyPickUpText (UserInterface|GetUserWidgetObject (Variables|Default|GetWidget))))
  (bind _output_get (Variables|Default|SetAs%20My%20Pick%20Up%20Text _asmy_pick_up_text))
  (Variables|/Game/blueprints/myUmg/myPickUpText.myPickUpText_C|SetpickUpText _output_get "장착 [T]")
  (Rendering|SetVisibility (Variables|Default|Getsm_fishingRod_2) false false))

(event Collision|EventActorBeginOverlap
  (params (OtherActor :type Actor%20Object%20Reference)))

(event EventTick
  (params (DeltaSeconds :type Float%20%28single-precision%29)))

(fn ConstructionScript)