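; Purchasable furniture actor that shows a prompt widget while something overlaps its sphere.
; Construction applies its custom mesh and fills its item info from custom image, text and price fields.
; It binds to the player character's buy event and, when in range, spawns a TempletePickUp at its arrow with that mesh and info, a pick-up prompt and negative AddEnergy.
; Overlaps are not filtered by actor, and no payment happens here.
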(event OnComponentBeginOverlap(Sphere)
  (params (OverlappedComponent :type Primitive%20Component%20Object%20Reference) (OtherActor :type Actor%20Object%20Reference) (OtherComp :type Primitive%20Component%20Object%20Reference) (OtherBodyIndex :type Integer) (bFromSweep :type Boolean) (SweepResult :type Hit%20Result%20Structure%20%28by%20ref%29))
  (Rendering|SetVisibility (Variables|Default|GetWidget) true false)
  (Variables|Default|Setin%20range%20? true))

(event OnComponentEndOverlap(Sphere)
  (params (OverlappedComponent :type Primitive%20Component%20Object%20Reference) (OtherActor :type Actor%20Object%20Reference) (OtherComp :type Primitive%20Component%20Object%20Reference) (OtherBodyIndex :type Integer))
  (Rendering|SetVisibility (Variables|Default|GetWidget) false false)
  (Variables|Default|Setin%20range%20? false))

(event Custom|buyFurniture
  (if (Variables|Default|Getin%20range%20?)
    (bind _returnvalue (Game|SpawnActorfromClass "/Game/blueprints/templetePickUp.templetePickUp_C" (Transformation|GetWorldTransform (Variables|Default|GetArrow)) "Undefined" 0 0))
    (Variables|/Game/blueprints/templetePickUp.templetePickUp_C|SetaddEnergy _returnvalue -0.5)
    (bind _output_get (Variables|/Game/blueprints/templetePickUp.templetePickUp_C|SetitemInfo _returnvalue (Variables|Default|GetitemInfo)))
    (Utilities|Struct|SetmembersininventoryStruct _output_get _returnvalue (Variables|Default|GetcustomImage) "줍기 [Q]" (Variables|Default|GetcustomActionText) (Variables|Default|GetcustomPrice) (Variables|Default|GetcustomPriceText))
    (Components|StaticMesh|SetStaticMesh (Variables|/Game/blueprints/templetePickUp.templetePickUp_C|GetStaticMesh _returnvalue) (Variables|Default|GetcustomStaticMesh))))

(event EventBeginPlay
  (bind _asmy_pick_up_text (Utilities|Casting|CastTomyPickUpText (UserInterface|GetUserWidgetObject (Variables|Default|GetWidget))))
  (bind _output_get (Variables|Default|SetAs%20My%20Pick%20Up%20Text _asmy_pick_up_text))
  (Variables|/Game/blueprints/myUmg/myPickUpText.myPickUpText_C|SetpickUpText _output_get (Variables|Default|GetcustomPickUpText))
  (bind _asmy_character (Utilities|Casting|CastTomyCharacter (Game|GetPlayerCharacter 0)))
  (bind _output_get_2 (Variables|Default|SetAs%20My%20Character _asmy_character))
  (EventDispatchers|BindEventtoBuyFurniture _output_get_2 (delegate Custom|buyFurniture)))

(event Collision|EventActorBeginOverlap
  (params (OtherActor :type Actor%20Object%20Reference)))

(event EventTick
  (params (DeltaSeconds :type Float%20%28single-precision%29)))

(fn ConstructionScript
  (Utilities|Struct|SetmembersininventoryStruct (Variables|Default|GetitemInfo) self (Variables|Default|GetcustomImage) (Variables|Default|GetcustomPickUpText) (Variables|Default|GetcustomActionText) (Variables|Default|GetcustomPrice) (Variables|Default|GetcustomPriceText))
  (Components|StaticMesh|SetStaticMesh (Variables|Default|GetStaticMesh) (Variables|Default|GetcustomStaticMesh)))