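; A spray can actor that recolors the player character's hair when used within range.
; Its construction script tints the can through a dynamic material instance using the actor's Color, and BeginPlay puts its Name in the widget text.
; Sphere overlaps toggle that widget and an InRange flag.
; It binds to the character's ChangeHair dispatcher and, if in range, applies Color to the character material's hairColor parameter.
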(event OnComponentBeginOverlap(Sphere)
  (params (OverlappedComponent :type Primitive%20Component%20Object%20Reference) (OtherActor :type Actor%20Object%20Reference) (OtherComp :type Primitive%20Component%20Object%20Reference) (OtherBodyIndex :type Integer) (bFromSweep :type Boolean) (SweepResult :type Hit%20Result%20Structure%20%28by%20ref%29))
  (Rendering|SetVisibility (Variables|Default|GetWidget) true false)
  (Variables|Default|Setin%20range%20? true))

(event OnComponentEndOverlap(Sphere)
  (params (OverlappedComponent :type Primitive%20Component%20Object%20Reference) (OtherActor :type Actor%20Object%20Reference) (OtherComp :type Primitive%20Component%20Object%20Reference) (OtherBodyIndex :type Integer))
  (Rendering|SetVisibility (Variables|Default|GetWidget) false false)
  (Variables|Default|Setin%20range%20? false))

(event Custom|changeHair_Event
  (if (Variables|Default|Getin%20range%20?)
    (Rendering|Material|SetVectorParameterValue (Variables|/Game/blueprints/myCharacter.myCharacter_C|Getdmi_character (stale EventBeginPlay _asmy_character)) "hairColor" (Variables|Default|Getcolor) :!class /Script/Engine.MaterialInstanceDynamic)))

(event EventBeginPlay
  (bind _asmy_pick_up_text (Utilities|Casting|CastTomyPickUpText (UserInterface|GetUserWidgetObject (Variables|Default|GetWidget))))
  (bind _output_get (Variables|Default|SetAs%20My%20Pick%20Up%20Text _asmy_pick_up_text))
  (Variables|/Game/blueprints/myUmg/myPickUpText.myPickUpText_C|SetpickUpText _output_get (Variables|Default|Getname))
  (bind _asmy_character (Utilities|Casting|CastTomyCharacter (Game|GetPlayerCharacter 0)))
  (bind _output_get_2 (Variables|Default|SetAs%20My%20Character _asmy_character))
  (EventDispatchers|AssignChangeHair _output_get_2 (delegate Custom|changeHair_Event)))

(event Collision|EventActorBeginOverlap
  (params (OtherActor :type Actor%20Object%20Reference)))

(event EventTick
  (params (DeltaSeconds :type Float%20%28single-precision%29)))

(fn ConstructionScript
  (Variables|Default|Setname (Variables|Default|Getname))
  (Variables|Default|Setcolor (Variables|Default|Getcolor))
  (bind _returnvalue (Rendering|Material|CreateDynamicMaterialInstance (Variables|Default|GetStaticMesh) 0 "/Game/materials/m_spray_Inst.m_spray_Inst" "None" :!class /Script/Engine.PrimitiveComponent))
  (bind _output_get (Variables|Default|Setdmi_sparay _returnvalue))
  (Rendering|Material|SetVectorParameterValue _output_get "canColor" (Variables|Default|Getcolor) :!class /Script/Engine.MaterialInstanceDynamic))