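; Sparrow creature that wanders at random until killed, then drops a steak pickup.
; While alive, Tick runs a random Delay, then AI-moves to a random reachable point nearby, tracking movement in IsMoving.
; Any damage kills it outright: collision turns off and the death animation plays.
; After a pause it spawns a TempletePickUp at DropLocation, configured as an edible, sellable steak, and destroys itself.
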(event EventBeginPlay)

(event Collision|EventActorBeginOverlap
  (params (OtherActor :type Actor%20Object%20Reference)))

(event EventTick
  (params (DeltaSeconds :type Float%20%28single-precision%29))
  (if (not (Variables|Default|Getdie%20?))
    (Utilities|FlowControl|Delay (Math|Random|RandomFloatinRange 1.0 3.0))
    (Variables|Default|Setis%20moving%20? true)
    (AI|AIMoveTo self (.RandomLocation (AI|Navigation|GetRandomReachablePointinRadius (Transformation|GetActorLocation) 5e+02 0 0)) 0 5.0 false
      (:OnSuccess
        _)
      (:OnFail
        _))
    (Variables|Default|Setis%20moving%20? false)))

(event Game|Damage|EventAnyDamage
  (params (Damage :type Float%20%28single-precision%29) (DamageType :type Damage%20Type%20Object%20Reference) (InstigatedBy :type Controller%20Object%20Reference) (DamageCauser :type Actor%20Object%20Reference))
  (Variables|Default|Setdie%20? true)
  (Collision|SetActorEnableCollision false)
  (Components|Animation|PlayAnimation (Variables|Character|GetMesh) "/Game/models/for_animal/Sparrow_Animations_Anim_Death.Sparrow_Animations_Anim_Death" false)
  (Utilities|FlowControl|Delay 5.0)
  (bind _returnvalue (Game|SpawnActorfromClass "/Game/blueprints/templetePickUp.templetePickUp_C" (Transformation|GetWorldTransform (Variables|Default|GetdropLocation)) "Undefined" 0 0))
  (bind _output_get (Variables|/Game/blueprints/templetePickUp.templetePickUp_C|SetitemInfo _returnvalue (Variables|Default|GetsparrowInfo)))
  (Utilities|Struct|SetmembersininventoryStruct _output_get _returnvalue "/Game/textures/steak.steak" "줍기 [Q]" "맛있게 먹기 ( +0.4 )" 150 "판매 (+150)")
  (Components|StaticMesh|SetStaticMesh (Variables|/Game/blueprints/templetePickUp.templetePickUp_C|GetStaticMesh _returnvalue) "/Game/models/steak/sm_steak.sm_steak")
  (Actor|DestroyActor))

(fn ConstructionScript)