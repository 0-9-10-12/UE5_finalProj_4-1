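; Player character Blueprint for a game with fishing, shooting, an inventory and money-based purchases.
; Enhanced Input events drive a rod/gun swap, fishing inside a trigger box, and an over-the-shoulder aim mode firing line-trace damage.
; Tick drains energy, sending the exhausted player to the house spawn with partial energy.
; Tagged capsule overlaps set a danger flag and handle shop and house entrances through camera-fade teleports.
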(event OnComponentBeginOverlap(CapsuleComponent)
  (params (OverlappedComponent :type Primitive%20Component%20Object%20Reference) (OtherActor :type Actor%20Object%20Reference) (OtherComp :type Primitive%20Component%20Object%20Reference) (OtherBodyIndex :type Integer) (bFromSweep :type Boolean) (SweepResult :type Hit%20Result%20Structure%20%28by%20ref%29))
  (Utilities|FlowControl|Sequence
    (:then_0
      (if (Components|ComponentHasTag OtherComp "test01")
        (Variables|Default|Setdanger true)))
    (:then_1
      (if (Components|ComponentHasTag OtherComp "shopIn")
        (CallFunction|CameraFadeOut)
        (Utilities|FlowControl|Delay 2.0)
        (Transformation|SetActorLocationAndRotation "-1430.000000,2880.000000,-2293.143607" "0.000000,-90.000000,0.000000")
        (Variables|Default|Setis%20shop%20? true)
        (CallFunction|CameraFadein)))
    (:then_2
      (if (Components|ComponentHasTag OtherComp "shopOut")
        (CallFunction|CameraFadeOut)
        (Utilities|FlowControl|Delay 2.0)
        (Transformation|SetActorLocationAndRotation "1010.000000,2150.000000,641.766122" "0.000000,90.000000,0.000000")
        (Variables|Default|Setis%20shop%20? false)
        (CallFunction|CameraFadein)))
    (:then_3
      (if (Components|ComponentHasTag OtherComp "houseIn")
        (CallFunction|CameraFadeOut)
        (Utilities|FlowControl|Delay 2.0)
        (Transformation|SetActorLocationAndRotation "440.000000,2020.000000,-2293.143604" "0.000000,90.000000,0.000000")
        (CallFunction|CameraFadein)))
    (:then_4
      (if (Components|ComponentHasTag OtherComp "houseOut")
        (CallFunction|CameraFadeOut)
        (Utilities|FlowControl|Delay 2.0)
        (Transformation|SetActorLocationAndRotation "-188.000000,82.000000,641.766063" "0.000000,90.000000,0.000000")
        (CallFunction|CameraFadein)))))

(event OnComponentEndOverlap(CapsuleComponent)
  (params (OverlappedComponent :type Primitive%20Component%20Object%20Reference) (OtherActor :type Actor%20Object%20Reference) (OtherComp :type Primitive%20Component%20Object%20Reference) (OtherBodyIndex :type Integer))
  (if (Components|ComponentHasTag OtherComp "test01")
    (Variables|Default|Setdanger false)))

(event Input|EnhancedActionEvents|EnhancedInputActionia_jump
  (params (ActionValue :type Boolean) (ElapsedSeconds :type Float%20%28double-precision%29) (TriggeredSeconds :type Float%20%28double-precision%29) (InputAction :type Input%20Action%20Object%20Reference :default "/Game/blueprints/myInput/ia_jump.ia_jump"))
  (:Triggered
    (if (!= (Variables|Default|GetmenuOpen) true)
      (Character|Jump))))

(event Input|EnhancedActionEvents|EnhancedInputActionia_action
  (params (ActionValue :type Boolean) (ElapsedSeconds :type Float%20%28double-precision%29) (TriggeredSeconds :type Float%20%28double-precision%29) (InputAction :type Input%20Action%20Object%20Reference :default "/Game/blueprints/myInput/ia_action.ia_action"))
  (bind _springarm (Variables|Default|GetSpringArm))
  (bind _returnvalue (Transformation|GetWorldLocation _springarm))
  (:Triggered
    (if (!= (Variables|Default|GetmenuOpen) true)
      (Utilities|FlowControl|Sequence
        (:then_0
          (if (Variables|Default|Gethas%20fish%20rod)
            (bind _returnvalue_2 (Actor|GetActorOfClass "/Game/blueprints/bp_fishingTriggerBox.bp_fishingTriggerBox_C"))
            (if (Collision|IsOverlappingActor _returnvalue_2 :!class /Script/Engine.Actor)
              (if (Variables|Default|Getreset%20fish)
                (Variables|Default|Setreset%20fish false)
                (goto _label Reset)
                (else
                  (Utilities|FlowControl|DoOnce false :!label _label
                    (:Completed
                      (Utilities|FlowControl|Sequence
                        (:then_0
                          (Variables|Default|Setenergy (- (Variables|Default|Getenergy) 0.1)))
                        (:then_1
                          (Rendering|SetVisibility (Variables|Default|Getsm_fishingRod_2) false false)
                          (Rendering|SetVisibility (Variables|Default|Getsm_fishingRod) true false)
                          (Rendering|SetVisibility (Variables|Default|Getsm_goldFish1) false false))
                        (:then_2
                          (Variables|Default|Setfish_animation true)
                          (Pawn|Components|CharacterMovement|DisableMovement (Variables|Character|GetCharacterMovement))
                          (Variables|Default|Setreset%20fish false)
                          (Utilities|FlowControl|Delay 4.33)
                          (Default|CallFishUI))))))))))
        (:then_1
          (if (Variables|Default|Getaim)
            (Animation|PlayAnimMontage "/Game/blueprints/myCharacterMontage.myCharacterMontage" 1.0 "fire")
            (bind (_outhit _returnvalue_3) (Collision|LineTraceByChannel _returnvalue (+ (* (Math|Vector|GetForwardVector _springarm) 1e+04) _returnvalue) "TraceTypeQuery1" false 0 "None"))
            (if _returnvalue_3
              (Effects|SpawnEmitteratLocation "/Game/StarterContent/Particles/P_Explosion.P_Explosion" (.Location (Collision|BreakHitResult _outhit)) "0, 0, 0" "0.500000,0.500000,0.500000")
              (Game|Damage|ApplyDamage (.HitActor (Collision|BreakHitResult _outhit)) 1e+02 0 0))))))))

(event Input|EnhancedActionEvents|EnhancedInputActionia_inventory
  (params (ActionValue :type Boolean) (ElapsedSeconds :type Float%20%28double-precision%29) (TriggeredSeconds :type Float%20%28double-precision%29) (InputAction :type Input%20Action%20Object%20Reference :default "/Game/blueprints/myInput/ia_inventory.ia_inventory"))
  (bind _hud (Variables|Default|GetHUD))
  (bind _hud_2 (Variables|Default|GetHUD))
  (bind _hud_3 (Variables|Default|GetHUD))
  (:Triggered
    (if (and (Variables|/Game/blueprints/myUmg/myUI.myUI_C|GetactivateInventory _hud_3) (!= (Variables|Default|Getinventory%20delay) true))
      (Utilities|FlowControl|FlipFlop
        (:A
          (Variables|/Game/blueprints/myUmg/myUI.myUI_C|SetinventoryVisible _hud_3 "Visible")
          (CallFunction|EnableMouseCursor)
          (UserInterface|Animation|PlayAnimation _hud_2 (Variables|/Game/blueprints/myUmg/myUI.myUI_C|GetmenuAnimation _hud_2) 0.0 1 "Forward" 1.0 false)
          (Variables|Default|Setinventory%20delay true)
          (Variables|Default|SetmenuOpen true))
        (:B
          (Variables|Default|Setinventory%20delay true)
          (UserInterface|Animation|PlayAnimation _hud (Variables|/Game/blueprints/myUmg/myUI.myUI_C|GetmenuAnimation _hud) 0.0 1 "Reverse" 1.0 false)
          (Utilities|FlowControl|Delay 0.5)
          (Variables|/Game/blueprints/myUmg/myUI.myUI_C|SetinventoryVisible _hud_3 "Hidden")
          (CallFunction|DisableMouseCursor)
          (Variables|Default|SetmenuOpen false)))
      (Utilities|FlowControl|Delay 0.5)
      (Variables|Default|Setinventory%20delay false))))

(event Input|EnhancedActionEvents|EnhancedInputActionia_pickItem
  (params (ActionValue :type Boolean) (ElapsedSeconds :type Float%20%28double-precision%29) (TriggeredSeconds :type Float%20%28double-precision%29) (InputAction :type Input%20Action%20Object%20Reference :default "/Game/blueprints/myInput/ia_pickItem.ia_pickItem"))
  (:Triggered
    (if (< (Utilities|Array|Length (Variables|/Game/blueprints/myUmg/myUI.myUI_C|GetinventoryStruct (Variables|Default|GetHUD))) 5)
      (Default|CallPickUpItem))))

(event Input|EnhancedActionEvents|EnhancedInputActionia_change
  (params (ActionValue :type Boolean) (ElapsedSeconds :type Float%20%28double-precision%29) (TriggeredSeconds :type Float%20%28double-precision%29) (InputAction :type Input%20Action%20Object%20Reference :default "/Game/blueprints/myInput/ia_change.ia_change"))
  (:Triggered
    (bind _returnvalue (Actor|GetActorOfClass "/Game/blueprints/bp_myGun.bp_myGun_C"))
    (if (Variables|/Game/blueprints/bp_myGun.bp_myGun_C|Getin%20range%20? _returnvalue)
      (Rendering|ToggleVisibility (Variables|/Script/Engine.StaticMeshActor|GetStaticMeshComponent _returnvalue) false)
      (Rendering|ToggleVisibility (Variables|/Game/blueprints/bp_myGun.bp_myGun_C|Getsm_fishingRod_2 _returnvalue) false)
      (Rendering|ToggleVisibility (Variables|Default|Getsm_fishingRod_2) false)
      (Rendering|ToggleVisibility (Variables|Default|Getsm_gun) false)
      (Utilities|FlowControl|FlipFlop
        (:A
          (Variables|Default|Sethas%20gun true)
          (Variables|Default|Sethas%20fish%20rod false))
        (:B
          (Variables|Default|Sethas%20gun false)
          (Variables|Default|Sethas%20fish%20rod true))))))

(event Input|EnhancedActionEvents|EnhancedInputActionia_aim
  (params (ActionValue :type Boolean) (ElapsedSeconds :type Float%20%28double-precision%29) (TriggeredSeconds :type Float%20%28double-precision%29) (InputAction :type Input%20Action%20Object%20Reference :default "/Game/blueprints/myInput/ia_aim.ia_aim"))
  (bind _has_gun (Variables|Default|Gethas%20gun))
  (:Triggered
    (if _has_gun
      (Utilities|FlowControl|DoOnce false :!label _label
        (:Completed
          (CallFunction|AimMode)))))
  (:Completed
    (if _has_gun
      (CallFunction|NaviMode)
      (goto _label Reset))))

(event Input|EnhancedActionEvents|EnhancedInputActionia_hair
  (params (ActionValue :type Boolean) (ElapsedSeconds :type Float%20%28double-precision%29) (TriggeredSeconds :type Float%20%28double-precision%29) (InputAction :type Input%20Action%20Object%20Reference :default "/Game/blueprints/myInput/ia_hair.ia_hair"))
  (bind _hud (Variables|Default|GetHUD))
  (:Triggered
    (if (>= (Variables|/Game/blueprints/myUmg/myUI.myUI_C|Getmoney _hud) 10)
      (Variables|/Game/blueprints/myUmg/myUI.myUI_C|Setmoney _hud (- (Variables|/Game/blueprints/myUmg/myUI.myUI_C|Getmoney _hud) 10))
      (Default|CallChangeHair))))

(event Input|EnhancedActionEvents|EnhancedInputActionia_buy
  (params (ActionValue :type Boolean) (ElapsedSeconds :type Float%20%28double-precision%29) (TriggeredSeconds :type Float%20%28double-precision%29) (InputAction :type Input%20Action%20Object%20Reference :default "/Game/blueprints/myInput/ia_buy.ia_buy"))
  (bind _hud (Variables|Default|GetHUD))
  (:Triggered
    (if (>= (Variables|/Game/blueprints/myUmg/myUI.myUI_C|Getmoney _hud) 15)
      (Variables|/Game/blueprints/myUmg/myUI.myUI_C|Setmoney _hud (- (Variables|/Game/blueprints/myUmg/myUI.myUI_C|Getmoney _hud) 15))
      (Default|CallBuyFurniture))))

(event EventBeginPlay
  (bind _returnvalue (UserInterface|CreateWidget "/Game/blueprints/myUmg/myUI.myUI_C"))
  (bind _output_get (Variables|Default|SetHUD _returnvalue))
  (UserInterface|Viewport|AddtoViewport _output_get 0)
  (Variables|Default|Sethas%20fish%20rod true)
  (Rendering|SetVisibility (Variables|Default|Getsm_fishingRod) false false)
  (Rendering|SetVisibility (Variables|Default|Getsm_goldFish1) false false)
  (Rendering|SetVisibility (Variables|Default|Getsm_gun1) false false)
  (Rendering|SetVisibility (Variables|Default|Getsm_gun) false false)
  (bind _returnvalue_2 (Rendering|Material|CreateDynamicMaterialInstance (Variables|Character|GetMesh) 0 "/Game/characterModel/Ch46_body_Inst.Ch46_body_Inst" "None" :!class /Script/Engine.PrimitiveComponent))
  (Variables|Default|Setdmi_character _returnvalue_2))

(event EventTick
  (params (DeltaSeconds :type Float%20%28single-precision%29))
  (Utilities|FlowControl|Sequence
    (:then_0
      (Variables|Default|Setspeed (Math|Vector|VectorLengthXY (Transformation|GetVelocity)))
      (if (<= (Variables|Default|Getenergy) 0.0)
        (Variables|Default|Setno%20energy true)
        (Utilities|FlowControl|DoOnce false :!label _label
          (:Completed
            (Utilities|FlowControl|Delay 3.0)
            (CallFunction|CameraFadeOut)
            (Utilities|FlowControl|Delay 2.0)
            (Variables|Default|Setenergy 0.8)
            (Transformation|SetActorLocationAndRotation "440.000000,2020.000000,-2293.143604" "0.000000,90.000000,0.000000")
            (CallFunction|CameraFadein)
            (goto _label Reset)))
        (else
          (Variables|Default|Setno%20energy false))))
    (:then_1
      (Variables|Default|Setenergy (- (Variables|Default|Getenergy) 0.0001)))))

(event EventDropAction
  (params (item%20to%20drop :type Actor%20Object%20Reference))
  (Variables|Default|SetmenuOpen true)
  (Animation|PlayAnimMontage "/Game/blueprints/myCharacterMontage.myCharacterMontage" -1.0 "pick")
  (Utilities|FlowControl|Delay 1.0)
  (Variables|Default|SetmenuOpen false)
  (Rendering|SetActorHiddenInGame item%20to%20drop false)
  (Collision|SetActorEnableCollision item%20to%20drop true)
  (Transformation|SetActorTransform item%20to%20drop (Transformation|GetWorldTransform (Variables|Default|GetdropLocation))))

(fn ConstructionScript)

(fn EnableMouseCursor
  (bind _returnvalue (Game|GetPlayerController 0))
  (Input|SetInputModeGameandUI _returnvalue (Variables|Default|GetHUD) "DoNotLock" true false)
  (Utilities|Casting|CastTomyCharacterHUD (HUD|GetHUD _returnvalue))
  (Variables|/Script/Engine.PlayerController|SetbShowMouseCursor _returnvalue true))

(fn DisableMouseCursor
  (bind _returnvalue (Game|GetPlayerController 0))
  (Input|SetInputModeGameOnly _returnvalue false)
  (Utilities|Casting|CastTomyCharacterHUD (HUD|GetHUD _returnvalue))
  (Variables|/Script/Engine.PlayerController|SetbShowMouseCursor _returnvalue false))

(fn CameraFadeOut
  (CameraFades|StartCameraFade :self (Variables|/Script/Engine.PlayerController|GetPlayerCameraManager (Game|GetPlayerController 0)) :ToAlpha 1.0 :Duration 1.5 :bHoldWhenFinished true)
  (return))

(fn CameraFadein
  (CameraFades|StartCameraFade :self (Variables|/Script/Engine.PlayerController|GetPlayerCameraManager (Game|GetPlayerController 0)) :FromAlpha 1.0 :Duration 1.5 :bHoldWhenFinished true))

(fn NaviMode
  (bind _returnvalue (Game|GetPlayerCameraManager 0))
  (bind _returnvalue_2 (Transformation|GetActorRotation))
  (bind _springarm (Variables|Default|GetSpringArm))
  (Rendering|SetVisibility (Variables|Default|Getsm_gun1) false false)
  (Variables|Default|Setaim false)
  (Variables|Default|SetbUseControllerRotationPitch false)
  (Variables|Default|SetbUseControllerRotationYaw false)
  (Variables|/Script/Engine.PlayerCameraManager|SetViewPitchMax _returnvalue 9e+01)
  (Variables|/Script/Engine.PlayerCameraManager|SetViewPitchMin _returnvalue -9e+01)
  (Variables|/Script/Engine.SpringArmComponent|SetTargetArmLength _springarm 5e+02)
  (Variables|/Script/Engine.SpringArmComponent|SetbEnableCameraLag _springarm true)
  (Variables|/Script/Engine.SpringArmComponent|SetbEnableCameraRotationLag _springarm true)
  (Animation|StopAnimMontage "/Game/blueprints/myCharacterMontage.myCharacterMontage")
  (Transformation|SetActorRotation (Math|Rotator|MakeRotator (.roll _returnvalue_2) 0.0 (.yaw _returnvalue_2))))

(fn AimMode
  (bind _returnvalue (Game|GetPlayerCameraManager 0))
  (bind _springarm (Variables|Default|GetSpringArm))
  (Rendering|SetVisibility (Variables|Default|Getsm_gun1) true false)
  (Variables|Default|Setaim true)
  (Variables|Default|SetbUseControllerRotationPitch true)
  (Variables|Default|SetbUseControllerRotationYaw true)
  (Variables|/Script/Engine.PlayerCameraManager|SetViewPitchMax _returnvalue 2e+01)
  (Variables|/Script/Engine.PlayerCameraManager|SetViewPitchMin _returnvalue -2e+01)
  (Variables|/Script/Engine.SpringArmComponent|SetTargetArmLength _springarm -25.0)
  (Variables|/Script/Engine.SpringArmComponent|SetbEnableCameraLag _springarm false)
  (Variables|/Script/Engine.SpringArmComponent|SetbEnableCameraRotationLag _springarm false)
  (Animation|PlayAnimMontage "/Game/blueprints/myCharacterMontage.myCharacterMontage" 1.0 "aim"))